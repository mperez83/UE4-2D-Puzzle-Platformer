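; FrogCharacter is a Paper2D playable frog form, apparently temporary, that gets around by hopping.
; Horizontal input on the ground fires a throttled upward impulse, while airborne input steers along X, and the jump gate resets on landing via Tick.
; CastSpell moves the Instigator to the frog's location, re-enables and possesses it, then destroys the frog.
; Flipbook animation and facing logic exist, but their update chain is disconnected.
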(event `self.ReceiveBeginPlay`)

(event `InputAxis|MoveRight`
  (params (AxisValue :type "Float (single-precision)"))
  (bind _charactermovement (`self.CharacterMovement`))
  ;[1 1 1] Handle movement
  (if (> AxisValue 0.0)
    (set `self.IsMovingRight` true)
    (if (`NavMovementComponent.IsMovingOnGround` _charactermovement) :!label _label
      (`/Engine/EditorBlueprintResources/StandardMacros.DoOnce` false :!label _label_2
        (:`Completed`
          (`CharacterMovementComponent.AddImpulse` _charactermovement (0.0 0.0 40000.0) false)
          (`KismetSystemLibrary.Delay` 0.4)
          (goto _label_2 :!via `Reset`)))
      (else
        (`self.AddMovementInput` (1.0 0.0 0.0) AxisValue)))
    (elif (< AxisValue 0.0)
      (set `self.IsMovingRight` false)
      (goto _label))))

(event `InputAction|Jump`
  (params (Key :type "Key Structure"))
  ;[1 1 1] Handle Jump
  (:`Pressed`
    (`/Engine/EditorBlueprintResources/StandardMacros.DoOnce` false :!label _label_3
      (:`Completed`
        (`self.Jump`)))))

(event `self.ReceiveTick`
  (params (DeltaSeconds :type "Float (single-precision)"))
  ;[1 1 1] Handle Jump
  (if (`NavMovementComponent.IsMovingOnGround` (`self.CharacterMovement`))
    (goto _label_3 :!via `Reset`)))

(event `InputAction|CastSpell`
  (params (Key :type "Key Structure"))
  (bind _returnvalue (`self.GetInstigator`))
  (:`Pressed`
    (`self.K2_SetActorLocation` _returnvalue (`self.K2_GetActorLocation`) false false)
    (`/Game/Blueprints/UtilityNodes.EnableActor` _returnvalue)
    (`/Game/Blueprints/UtilityNodes.ControllerChangePossession` (`GameplayStatics.GetPlayerController` 0) _returnvalue)
    (`self.K2_DestroyActor`)))

(event `UpdateAnimation`
  (bind (_returnvalue_x _returnvalue_y _returnvalue_z) (`KismetMathLibrary.BreakVector` (`self.GetVelocity`)))
  ;[1 1 1] Handle Animation
  (if (`self.AnimationLocked`)
    _
    (elif (`NavMovementComponent.IsMovingOnGround` (`self.CharacterMovement`))
      (`|ExecutionSequence`
        (:`then_0`
          (`PaperFlipbookComponent.SetFlipbook` (`self.Sprite`) (select `bool` (> (`KismetMathLibrary.VSize` (`self.GetVelocity`)) 0.0) :`false` "/Game/Art/Sprites/PlayerSprites/Placeholder/Idle/FB_Player_Idle.FB_Player_Idle" :`true` "/Game/Art/Sprites/PlayerSprites/Placeholder/Running/FB_Player_Run.FB_Player_Run" :!type "PaperFlipbook Object Reference")))
        (:`then_1`
          (goto _label_4 :!via `Reset`)))
      (elif (>= _returnvalue_z 0.0)
        (`/Engine/EditorBlueprintResources/StandardMacros.DoOnce` false :!label _label_4
          (:`Completed`
            (`PaperFlipbookComponent.SetFlipbook` (`self.Sprite`) "/Game/Art/Sprites/PlayerSprites/Placeholder/JumpAscending/FB_Player_JumpAscending.FB_Player_JumpAscending")))
        (else
          (`PaperFlipbookComponent.SetFlipbook` (`self.Sprite`) "/Game/Art/Sprites/PlayerSprites/Placeholder/JumpDescending/FB_Player_JumpDescending.FB_Player_JumpDescending"))))))

(event `PlayFullAnimation`
  (params (FlipbookToPlay :type "PaperFlipbook Object Reference"))
  ;[1 1 1] Handle Animation
  (set `self.AnimationLocked` true)
  (`PaperFlipbookComponent.SetFlipbook` (`self.Sprite`) FlipbookToPlay)
  (`KismetSystemLibrary.Delay` (`PaperFlipbook.GetTotalDuration` FlipbookToPlay))
  (set `self.AnimationLocked` false))

(fn `UserConstructionScript`)