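; Spell_Fireball is a spell Blueprint that implements the CastSpell event for a fireball attack, branching on SpellLevel.
; Level 1 spawns a Fireball actor at the player character's transform, with the player as instigator and horizontal velocity signed by the facing flag IsMovingRight.
; Levels 2 and 3 are placeholders that only print debug strings.
; The construction script only calls its parent.
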(event `/Game/Blueprints/Spells/Spell_Base_Interface.CastSpell`
  (bind _playercharacterref (`self.PlayerCharacterRef`))
  (switch `int` (`self.SpellLevel`)
    (:`1`
      (`|SpawnActorFromClass` "/Game/Blueprints/Spells/Fireball.Fireball_C" (`self.GetTransform` _playercharacterref) "Undefined" "OverrideRootScale" null (`KismetMathLibrary.MakeVector` (`KismetMathLibrary.SelectFloat` 20.0 -20.0 (`/Game/Blueprints/PlayerCharacter/PlayerCharacter.IsMovingRight` _playercharacterref))) _playercharacterref))
    (:`2`
      (`KismetSystemLibrary.PrintString` "SUPER FIREBALL!!!"))
    (:`3`
      (`KismetSystemLibrary.PrintString` "MEGA FIREBALL!!!!!!!!!"))))

(fn `UserConstructionScript`
  (`parent.UserConstructionScript`))