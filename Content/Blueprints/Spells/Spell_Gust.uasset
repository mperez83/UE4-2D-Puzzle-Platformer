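; Gust spell Blueprint that makes the player character dash when cast.
; CastSpell branches on the spell's level, from one to three, with higher levels giving a longer and faster dash.
; Each level checks the cast condition, runs the standard cast with the player cast flipbook, then calls StartDash on the player character.
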(event `/Game/Blueprints/Spells/Spell_Base_Interface.CastSpell`
  (switch `int` (`.Level_30_B9279FCB4EFC0C048953E5B782B10EC9` (break `/Game/Blueprints/Spells/Struct_Spells` (`self.GetSpellInfo`)))
    (:`1`
      (if (`self.GetIfCanCastSpell`)
        (`self.StandardCastSpell` "/Game/Art/Sprites/PlayerSprites/Placeholder/Cast/FB_Player_Cast.FB_Player_Cast")
        (`/Game/Blueprints/PlayerCharacter/PlayerCharacter.StartDash` (`self.PlayerCharacterRef`) 0.25 1500.0)))
    (:`2`
      (if (`self.GetIfCanCastSpell`)
        (`self.StandardCastSpell` "/Game/Art/Sprites/PlayerSprites/Placeholder/Cast/FB_Player_Cast.FB_Player_Cast")
        (`/Game/Blueprints/PlayerCharacter/PlayerCharacter.StartDash` (`self.PlayerCharacterRef`) 0.35 2000.0)))
    (:`3`
      (if (`self.GetIfCanCastSpell`)
        (`self.StandardCastSpell` "/Game/Art/Sprites/PlayerSprites/Placeholder/Cast/FB_Player_Cast.FB_Player_Cast")
        (`/Game/Blueprints/PlayerCharacter/PlayerCharacter.StartDash` (`self.PlayerCharacterRef`) 0.5 4000.0)))))

(fn `UserConstructionScript`
  (`parent.UserConstructionScript`))