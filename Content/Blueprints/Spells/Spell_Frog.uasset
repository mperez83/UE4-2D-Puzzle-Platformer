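; Frog spell that turns the player into a frog by swapping the controlled pawn.
; On cast, if casting is allowed, it subtracts the spell's cost from the player's spell uses and increments its cast count in the game instance's Spells array.
; It then disables the player character, spawns a FrogCharacter at the same transform with the player as Instigator, and hands player controller possession to the frog.
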(event `/Game/Blueprints/Spells/Spell_Base_Interface.CastSpell`
  (bind _spellinfo (`self.GetSpellInfo`))
  (bind _playercharacterref (`self.PlayerCharacterRef`))
  (cast `/Game/Blueprints/PlayerCharacter/PlayerCharacter` (`Controller.K2_GetPawn` (`GameplayStatics.GetPlayerController` 0)))
  (if (`self.GetIfCanCastSpell`)
    (`/Game/Blueprints/PlayerCharacter/PlayerCharacter.SubtractSpellUses` (`self.PlayerCharacterRef`) (`.Cost_32_4B608AD6462F395DA2F667ADA4B38332` (break `/Game/Blueprints/Spells/Struct_Spells` (`self.GetSpellInfo`))))
    (bind _structout (setmembers `/Game/Blueprints/Spells/Struct_Spells` :`StructRef` _spellinfo :`NumberOfTimesCast` (+ (`.NumberOfTimesCast_13_BA7B903A48F09F884C938F8D5622A345` (break `/Game/Blueprints/Spells/Struct_Spells` _spellinfo)) 1)))
    (`KismetArrayLibrary.Array_Set` (`/Game/Blueprints/2DGameInstance.Spells` (`self.2DGameInstance`)) (`self.SpellIndex`) _structout)
    (`/Game/Blueprints/UtilityNodes.DisableActor` _playercharacterref)
    (bind _returnvalue (`|SpawnActorFromClass` "/Game/Blueprints/PlayerCharacter/FrogCharacter.FrogCharacter_C" (`self.GetTransform` _playercharacterref) "Undefined" "OverrideRootScale" null _playercharacterref))
    (`/Game/Blueprints/UtilityNodes.ControllerChangePossession` (`GameplayStatics.GetPlayerController` 0) _returnvalue)))

(fn `UserConstructionScript`
  (`parent.UserConstructionScript`))