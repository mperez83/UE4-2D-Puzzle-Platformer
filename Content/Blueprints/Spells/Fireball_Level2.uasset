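; Level 2 fireball spell projectile that destroys burnable walls and explodes on contact.
; Each tick it moves by its Velocity offset without sweeping or delta-time scaling.
; Overlapping any actor other than its Instigator destroys that actor if it is a BurnableWall, then destroys the fireball and spawns a scaled-up Explosion at its transform.
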(event `self.ReceiveTick`
  (params (DeltaSeconds :type "Float (single-precision)"))
  (`self.K2_AddActorWorldOffset` (`self.Velocity`)))

(event `self.ReceiveActorBeginOverlap`
  (params (OtherActor :type "Actor Object Reference"))
  (if (!= OtherActor (`self.Instigator`))
    (`|ExecutionSequence`
      (:`then_0`
        (bind _asburnable_wall (cast `/Game/Blueprints/LevelEntities/BurnableWall` OtherActor))
        (`self.K2_DestroyActor` _asburnable_wall))
      (:`then_1`
        (`self.K2_DestroyActor`)
        (`|SpawnActorFromClass` "/Game/Blueprints/Spells/Explosion.Explosion_C" (`self.GetTransform`) "Undefined" "OverrideRootScale" null 10.0 null)))))

(fn `UserConstructionScript`)