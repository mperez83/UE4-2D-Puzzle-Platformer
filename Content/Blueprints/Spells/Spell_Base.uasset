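; Spell_Base is a base Blueprint for player spells.
; On BeginPlay it caches references to the PlayerCharacter pawn and the 2DGameInstance, stopping if a cast fails.
; GetIfCanCastSpell checks whether the player's remaining spell uses cover the cost stored in SpellInfo.
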(event `self.ReceiveBeginPlay`
  (bind _asplayer_character (cast `/Game/Blueprints/PlayerCharacter/PlayerCharacter` (`GameplayStatics.GetPlayerPawn` 0)))
  (set `self.PlayerCharacterRef` _asplayer_character)
  (bind _as2dgame_instance (cast `/Game/Blueprints/2DGameInstance` (`GameplayStatics.GetGameInstance`)))
  (set `self.2DGameInstance` _as2dgame_instance))

(fn `GetIfCanCastSpell`
  (returns (ReturnValue :type Boolean))
  (return (>= (`/Game/Blueprints/PlayerCharacter/PlayerCharacter.NumberOfSpellUsesLeft` (`self.PlayerCharacterRef`)) (`.SpellCost_24_4B608AD6462F395DA2F667ADA4B38332` (break `/Game/Blueprints/Spells/Struct_Spells` (`self.SpellInfo`))))))

(fn `UserConstructionScript`)