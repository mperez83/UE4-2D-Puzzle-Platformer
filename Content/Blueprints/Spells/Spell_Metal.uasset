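; Metal spell that toggles the player into a tinted, heavy metal form, locking spell swapping until it is cast again.
; Entering checks castability, spends uses, plays the cast flipbook, halts movement, raises gravity and applies an upward impulse; exiting is free.
; Each spell level repeats the toggle with lighter penalties: level 1 roots the player, level 2 allows slow walking without jumping, level 3 keeps speed and jump with milder gravity.
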(event `/Game/Blueprints/Spells/Spell_Base_Interface.CastSpell`
  (bind _playercharacterref (`self.PlayerCharacterRef`))
  (bind _playercharacterref_2 (`self.PlayerCharacterRef`))
  (bind _playercharacterref_3 (`self.PlayerCharacterRef`))
  (bind _playercharacterref_4 (`self.PlayerCharacterRef`))
  (bind _playercharacterref_5 (`self.PlayerCharacterRef`))
  (bind _playercharacterref_6 (`self.PlayerCharacterRef`))
  (bind _playercharacterref_7 (`self.PlayerCharacterRef`))
  (bind _playercharacterref_8 (`self.PlayerCharacterRef`))
  (bind _playercharacterref_9 (`self.PlayerCharacterRef`))
  (bind _charactermovement (`Character.CharacterMovement` _playercharacterref_9))
  (bind _charactermovement_2 (`Character.CharacterMovement` _playercharacterref_5))
  (bind _charactermovement_3 (`Character.CharacterMovement` _playercharacterref))
  (switch `int` (`.SpellLevel_11_B9279FCB4EFC0C048953E5B782B10EC9` (break `/Game/Blueprints/Spells/Struct_Spells` (`self.SpellInfo`)))
    (:`1`
      (if (`/Game/Blueprints/PlayerCharacter/PlayerCharacter.IsMetal` _playercharacterref_7)
        (set `/Game/Blueprints/PlayerCharacter/PlayerCharacter.IsMetal` false _playercharacterref_7)
        (set `/Game/Blueprints/PlayerCharacter/PlayerCharacter.CanSwapSpells` true _playercharacterref_7)
        (set `CharacterMovementComponent.GravityScale` 4.0 (`Character.CharacterMovement` _playercharacterref_3))
        (`/Game/Blueprints/PlayerCharacter/PlayerCharacter.SetNewSpeedScale` _playercharacterref_3 1.0)
        (`/Game/Blueprints/PlayerCharacter/PlayerCharacter.SetNewJumpPowerScale` _playercharacterref_3 1.0)
        (`PaperFlipbookComponent.SetSpriteColor` (`PaperCharacter.Sprite` _playercharacterref_3) (struct :`R` 1.0 :`G` 1.0 :`B` 1.0 :`A` 1.0))
        (elif (`self.GetIfCanCastSpell`)
          (`/Game/Blueprints/PlayerCharacter/PlayerCharacter.SubtractSpellUses` _playercharacterref_7 (`.SpellCost_24_4B608AD6462F395DA2F667ADA4B38332` (break `/Game/Blueprints/Spells/Struct_Spells` (`self.SpellInfo`))))
          (`/Game/Blueprints/PlayerCharacter/PlayerCharacter.PlayFullAnimation` _playercharacterref_7 "/Game/Art/Sprites/PlayerSprites/Placeholder/Cast/FB_Player_Cast.FB_Player_Cast")
          (set `/Game/Blueprints/PlayerCharacter/PlayerCharacter.IsMetal` true _playercharacterref_7)
          (set `/Game/Blueprints/PlayerCharacter/PlayerCharacter.CanSwapSpells` false _playercharacterref_7)
          (`MovementComponent.StopMovementImmediately` _charactermovement)
          (set `CharacterMovementComponent.GravityScale` 10.0 _charactermovement)
          (`CharacterMovementComponent.AddImpulse` _charactermovement (0.0 0.0 150000.0) false)
          (`/Game/Blueprints/PlayerCharacter/PlayerCharacter.SetNewSpeedScale` _playercharacterref_9 0.0)
          (`/Game/Blueprints/PlayerCharacter/PlayerCharacter.SetNewJumpPowerScale` _playercharacterref_9 0.0)
          (`PaperFlipbookComponent.SetSpriteColor` (`PaperCharacter.Sprite` _playercharacterref_9) (struct :`B` 1.0 :`A` 1.0)))))
    (:`2`
      (if (`/Game/Blueprints/PlayerCharacter/PlayerCharacter.IsMetal` _playercharacterref_4)
        (set `/Game/Blueprints/PlayerCharacter/PlayerCharacter.IsMetal` false _playercharacterref_4)
        (set `/Game/Blueprints/PlayerCharacter/PlayerCharacter.CanSwapSpells` true _playercharacterref_4)
        (set `CharacterMovementComponent.GravityScale` 4.0 (`Character.CharacterMovement` _playercharacterref_6))
        (`/Game/Blueprints/PlayerCharacter/PlayerCharacter.SetNewSpeedScale` _playercharacterref_6 1.0)
        (`/Game/Blueprints/PlayerCharacter/PlayerCharacter.SetNewJumpPowerScale` _playercharacterref_6 1.0)
        (`PaperFlipbookComponent.SetSpriteColor` (`PaperCharacter.Sprite` _playercharacterref_6) (struct :`R` 1.0 :`G` 1.0 :`B` 1.0 :`A` 1.0))
        (elif (`self.GetIfCanCastSpell`)
          (`/Game/Blueprints/PlayerCharacter/PlayerCharacter.SubtractSpellUses` _playercharacterref_4 (`.SpellCost_24_4B608AD6462F395DA2F667ADA4B38332` (break `/Game/Blueprints/Spells/Struct_Spells` (`self.SpellInfo`))))
          (`/Game/Blueprints/PlayerCharacter/PlayerCharacter.PlayFullAnimation` _playercharacterref_4 "/Game/Art/Sprites/PlayerSprites/Placeholder/Cast/FB_Player_Cast.FB_Player_Cast")
          (set `/Game/Blueprints/PlayerCharacter/PlayerCharacter.IsMetal` true _playercharacterref_4)
          (set `/Game/Blueprints/PlayerCharacter/PlayerCharacter.CanSwapSpells` false _playercharacterref_4)
          (`MovementComponent.StopMovementImmediately` _charactermovement_2)
          (set `CharacterMovementComponent.GravityScale` 10.0 _charactermovement_2)
          (`CharacterMovementComponent.AddImpulse` _charactermovement_2 (0.0 0.0 150000.0) false)
          (`/Game/Blueprints/PlayerCharacter/PlayerCharacter.SetNewSpeedScale` _playercharacterref_5 0.25)
          (`/Game/Blueprints/PlayerCharacter/PlayerCharacter.SetNewJumpPowerScale` _playercharacterref_5 0.0)
          (`PaperFlipbookComponent.SetSpriteColor` (`PaperCharacter.Sprite` _playercharacterref_5) (struct :`G` 0.25 :`B` 1.0 :`A` 1.0)))))
    (:`3`
      (if (`/Game/Blueprints/PlayerCharacter/PlayerCharacter.IsMetal` _playercharacterref_2)
        (set `/Game/Blueprints/PlayerCharacter/PlayerCharacter.IsMetal` false _playercharacterref_2)
        (set `/Game/Blueprints/PlayerCharacter/PlayerCharacter.CanSwapSpells` true _playercharacterref_2)
        (set `CharacterMovementComponent.GravityScale` 4.0 (`Character.CharacterMovement` _playercharacterref_8))
        (`PaperFlipbookComponent.SetSpriteColor` (`PaperCharacter.Sprite` _playercharacterref_8) (struct :`R` 1.0 :`G` 1.0 :`B` 1.0 :`A` 1.0))
        (elif (`self.GetIfCanCastSpell`)
          (`/Game/Blueprints/PlayerCharacter/PlayerCharacter.SubtractSpellUses` _playercharacterref_2 (`.SpellCost_24_4B608AD6462F395DA2F667ADA4B38332` (break `/Game/Blueprints/Spells/Struct_Spells` (`self.SpellInfo`))))
          (`/Game/Blueprints/PlayerCharacter/PlayerCharacter.PlayFullAnimation` _playercharacterref_2 "/Game/Art/Sprites/PlayerSprites/Placeholder/Cast/FB_Player_Cast.FB_Player_Cast")
          (set `/Game/Blueprints/PlayerCharacter/PlayerCharacter.IsMetal` true _playercharacterref_2)
          (set `/Game/Blueprints/PlayerCharacter/PlayerCharacter.CanSwapSpells` false _playercharacterref_2)
          (`MovementComponent.StopMovementImmediately` _charactermovement_3)
          (set `CharacterMovementComponent.GravityScale` 6.0 _charactermovement_3)
          (`CharacterMovementComponent.AddImpulse` _charactermovement_3 (0.0 0.0 150000.0) false)
          (`PaperFlipbookComponent.SetSpriteColor` (`PaperCharacter.Sprite` _playercharacterref) (struct :`G` 1.0 :`B` 1.0 :`A` 1.0)))))))

(fn `UserConstructionScript`
  (`parent.UserConstructionScript`))