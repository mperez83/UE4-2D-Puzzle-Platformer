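; Game instance for a 2D game that holds the master Spells array, tracking which spells are known and at what level.
; Known spells are spawned as actors carrying their spell struct, to fill the player's spell list.
; Learning a spell marks it known and spawns its actor into the PlayerCharacter's list.
; Upgrades respect max level, only raise it unless forced, and copy the updated struct into the matching player spell actor.
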(fn `GetSpellStructFromName`
  (params (SpellName :type "/Game/Blueprints/Spells/E_Spells Enum" :default "NewEnumerator0"))
  (returns (FoundSpell :type Boolean) (FoundSpellStruct :type "/Game/Blueprints/Spells/Struct_Spells Structure") (FoundSpellIndex :type Integer))
  (for (_array_element _array_index) (`self.Spells`)
    (if (== SpellName (`.SpellName_25_615B02EB4BC0E96BD152EC8655FBD2B7` (break `/Game/Blueprints/Spells/Struct_Spells` _array_element)))
      (return true _array_element _array_index)))
  (return false (struct) -1))

(fn `LearnNewSpell`
  (params (SpellName :type "/Game/Blueprints/Spells/E_Spells Enum" :default "NewEnumerator0"))
  (bind (_foundspell _foundspellstruct _foundspellindex) (`self.GetSpellStructFromName` SpellName))
  (bind (_spellname _spellclass _isknown) (break `/Game/Blueprints/Spells/Struct_Spells` _foundspellstruct))
  (if (not _isknown)
    (bind _structout (setmembers `/Game/Blueprints/Spells/Struct_Spells` :`StructRef` _foundspellstruct :`IsKnown` true))
    (`KismetArrayLibrary.Array_Set` (`self.Spells`) _foundspellindex _structout)
    (bind _returnvalue (`|SpawnActorFromClass` _spellclass (`KismetMathLibrary.MakeTransform` (0.0 0.0 0.0)) "Undefined" "OverrideRootScale" null _structout null))
    (bind _asplayer_character (cast `/Game/Blueprints/PlayerCharacter/PlayerCharacter` (`GameplayStatics.GetPlayerCharacter` 0)))
    (`KismetArrayLibrary.Array_Add` (`/Game/Blueprints/PlayerCharacter/PlayerCharacter.Spells` _asplayer_character) _returnvalue)))

(fn `PopulatePlayerSpells`
  (params (PlayerSpells :type "Array of /Game/Blueprints/Spells/Spell_Base Object Reference"))
  (for _array_element (`self.Spells`)
    (bind ((`SpellName_25_615B02EB4BC0E96BD152EC8655FBD2B7` _spellname) (`SpellClass_17_6AF9060347637B8F7670BE81A46D8C7D` _spellclass) (`IsKnown_15_2930CA3B45CB201012786988AAE34E82` _isknown)) (break `/Game/Blueprints/Spells/Struct_Spells` _array_element))
    (if _isknown
      (bind _returnvalue (`|SpawnActorFromClass` _spellclass (`KismetMathLibrary.MakeTransform` (0.0 0.0 0.0)) "Undefined" "OverrideRootScale" null _array_element null))
      (`KismetArrayLibrary.Array_Add` PlayerSpells _returnvalue))))

(fn `RefreshSpellInfoInPlayer`
  (params (SpellInfoToRefresh :type "/Game/Blueprints/Spells/Struct_Spells Structure"))
  (bind _asplayer_character (cast `/Game/Blueprints/PlayerCharacter/PlayerCharacter` (`GameplayStatics.GetPlayerPawn` 0)))
  (for _array_element (`/Game/Blueprints/PlayerCharacter/PlayerCharacter.Spells` _asplayer_character)
    (if (== (`.SpellName_25_615B02EB4BC0E96BD152EC8655FBD2B7` (break `/Game/Blueprints/Spells/Struct_Spells` (`/Game/Blueprints/Spells/Spell_Base.SpellInfo` _array_element))) (`.SpellName_25_615B02EB4BC0E96BD152EC8655FBD2B7` (break `/Game/Blueprints/Spells/Struct_Spells` SpellInfoToRefresh)))
      (set `/Game/Blueprints/Spells/Spell_Base.SpellInfo` SpellInfoToRefresh _array_element))))

(fn `Upgrade Spell Level`
  (params (SpellName :type "/Game/Blueprints/Spells/E_Spells Enum" :default "NewEnumerator0") (NewSpellLevel :type Integer) (ForceOverride :type Boolean))
  (locals (TempSpellLevel :type Integer))
  (bind (_foundspell _foundspellstruct _foundspellindex) (`self.GetSpellStructFromName` SpellName))
  (bind ((`IsKnown_15_2930CA3B45CB201012786988AAE34E82` _isknown) (`SpellLevel_11_B9279FCB4EFC0C048953E5B782B10EC9` _spelllevel) (`MaxSpellLevel_21_EDAB05B54A8ACFD03203EA806DC7021B` _maxspelllevel)) (break `/Game/Blueprints/Spells/Struct_Spells` _foundspellstruct))
  (if _isknown
    (bind _output_get (set `local.TempSpellLevel` NewSpellLevel))
    (if (<= _output_get _maxspelllevel)
      (if (or (> (`local.TempSpellLevel`) _spelllevel) ForceOverride)
        (bind _structout (setmembers `/Game/Blueprints/Spells/Struct_Spells` :`StructRef` _foundspellstruct :`SpellLevel` (`local.TempSpellLevel`)))
        (`KismetArrayLibrary.Array_Set` (`self.Spells`) _foundspellindex _structout)
        (`self.RefreshSpellInfoInPlayer` _structout)))))