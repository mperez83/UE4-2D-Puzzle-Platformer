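; NarrativeBubble is a speech bubble actor that shows a speaker's conversation lines one at a time through a SpeechBubble widget.
; BeginPlay shows the first line and enables input, so releasing CycleConversation advances through the string array.
; Tick keeps the widget at a fixed world offset from a valid Speaker, whose presence sets the arrow's visibility.
; After the last line it disables input, triggers NextSpeaker on an owning ConversationStarterZone and destroys itself.
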(event `InputAction|CycleConversation`
  (params (Key :type "Key Structure"))
  (:`Released`
    (`self.DisplayNextMessage`)))

(event `self.ReceiveBeginPlay`
  ;[1 1 1] Set Start Message Text
  (bind _asspeech_bubble (cast `/Game/Blueprints/UserInterface/Widgets/SpeechBubble` (`WidgetComponent.GetUserWidgetObject` (`self.Widget`))))
  (set `self.SpeechBubbleActor` _asspeech_bubble)
  (`self.DisplayNextMessage`)
  (`self.EnableInput` (`GameplayStatics.GetPlayerController` 0))
  ;[1 1 1] Setup Speaker
  (`/Engine/EditorBlueprintResources/StandardMacros.IsValid` (`self.Speaker`)
    (:`Is Valid`
      (`self.SetupSpeaker` true))
    (:`Is Not Valid`
      (`self.SetupSpeaker` false))))

(event `self.ReceiveTick`
  (params (DeltaSeconds :type "Float (single-precision)"))
  (bind _speaker (`self.Speaker`))
  ;[1 1 1] Tick: Follow Speaker         TODO: Dynamic Location
  (`/Engine/EditorBlueprintResources/StandardMacros.IsValid` _speaker ; if valid, update to follow the speaker
    (:`Is Valid`
      (`SceneComponent.K2_SetWorldLocation` (`self.Widget`) (`KismetMathLibrary.MakeVector` (+ (.x (`self.K2_GetActorLocation` _speaker)) 150.0) (- (.y (`self.K2_GetActorLocation` _speaker)) 5.0) (+ (.z (`self.K2_GetActorLocation` _speaker)) 200.0)) false false))))

(fn `DisplayNextMessage`
  (bind _returnvalue (`self.GetOwner`))
  (bind _conversationstringsarray (`self.ConversationStringsArray`))
  (bind _conversationstringindex (`self.ConversationStringIndex`))
  (if (`KismetArrayLibrary.Array_IsValidIndex` _conversationstringsarray _conversationstringindex)
    (bind _output_get (set `self.CurrentMessage` (`|GetArrayItem` _conversationstringsarray _conversationstringindex)))
    (`TextBlock.SetText` (`/Game/Blueprints/UserInterface/Widgets/SpeechBubble.Message` (`self.SpeechBubbleActor`)) (`KismetTextLibrary.Conv_StringToText` _output_get))
    (set `self.ConversationStringIndex` (+ _conversationstringindex 1))
    (else
      ;[1 1 1] Speaker is Done, If in a ConversationStarterZone start the Next Speaker
      (`self.DisableInput` (`GameplayStatics.GetPlayerController` 0))
      (`/Engine/EditorBlueprintResources/StandardMacros.IsValid` _returnvalue
        (:`Is Valid`
          (bind _asconversation_starter_zone (cast `/Game/Blueprints/NarrativeUI/ConversationStarterZone` _returnvalue))
          (`/Game/Blueprints/NarrativeUI/ConversationStarterZone.NextSpeaker` _asconversation_starter_zone))
        (:`Is Not Valid`
          _))
      (`self.K2_DestroyActor`))))

(fn `SetupSpeaker`
  (params (HasSpeaker :type Boolean))
  (bind _speakerarrow (`self.SpeakerArrow`))
  (if HasSpeaker
    (`KismetSystemLibrary.PrintString` "Has an Owner")
    (`SceneComponent.SetVisibility` _speakerarrow true false)
    (else
      (`KismetSystemLibrary.PrintString` "Has NO Owner")
      (`SceneComponent.SetVisibility` _speakerarrow false false))))

(fn `UserConstructionScript`)